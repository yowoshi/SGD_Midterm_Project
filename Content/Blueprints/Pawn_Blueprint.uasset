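; Player pawn that follows the mouse cursor, with a pause menu toggle.
; Each tick it yaws to face the cursor's trace hit, and while left mouse is held it moves forward through FloatingPawnMovement until within a short distance of that point.
; Escape flip-flops a Pause widget and the game's paused state.
; A touch-based movement branch exists but is never executed.
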(event `self.ReceiveBeginPlay`
  ;[0.4746 0.421 1] Moves Pawn to Mouse Location
  (set `PlayerController.bShowMouseCursor` true (`GameplayStatics.GetPlayerController` 0))
  (set `self.isClicked` false))

(event `Key|LeftMouseButton`
  (params (Key :type "Key Structure"))
  ;[0.4746 0.421 1] Moves Pawn to Mouse Location
  (:`Pressed`
    (set `self.isClicked` true))
  (:`Released`
    (set `self.isClicked` false)))

(event `self.ReceiveTick`
  (params (DeltaSeconds :type "Float (single-precision)"))
  (bind _returnvalue (`self.K2_GetActorLocation`))
  (bind _hitresult (`PlayerController.GetHitResultUnderCursorByChannel` (`GameplayStatics.GetPlayerController` 0) "TraceTypeQuery1" true))
  (bind (_returnvalue_roll _returnvalue_pitch _returnvalue_yaw) (`KismetMathLibrary.BreakRotator` (`KismetMathLibrary.FindLookAtRotation` _returnvalue (`.Location` (`GameplayStatics.BreakHitResult` _hitresult)))))
  ;[0.3571 0.9061 1] Update Pawn to Face Mouse
  (`SceneComponent.K2_SetWorldRotation` (`self.DefaultSceneRoot`) (`KismetMathLibrary.MakeRotator` 0.0 0.0 _returnvalue_yaw) false false)
  ;[0.4746 0.421 1] Moves Pawn to Mouse Location
  (if (and (`self.isClicked`) (> (`KismetMathLibrary.Vector_Distance` _returnvalue (`.Location` (`GameplayStatics.BreakHitResult` _hitresult))) 100.0))
    (`PawnMovementComponent.AddInputVector` (`self.FloatingPawnMovement`) (* (`KismetMathLibrary.Conv_RotatorToVector` (`SceneComponent.K2_GetComponentRotation` (`Actor.RootComponent` (`GameplayStatics.GetPlayerPawn` 0)))) 0.75) true)))

(event `Key|Escape` :paused true
  (params (Key :type "Key Structure"))
  ;[1 0.9295 0.3112] Pause
  (:`Pressed`
    (`/Engine/EditorBlueprintResources/StandardMacros.FlipFlop`
      (:`A`
        (bind _returnvalue (`|CreateWidget` "/Game/Widget/Pause.Pause_C"))
        (`UserWidget.AddToViewport` _returnvalue 0)
        (`GameplayStatics.SetGamePaused` true))
      (:`B`
        (`Widget.RemoveFromParent` _returnvalue)
        (`GameplayStatics.SetGamePaused` false)))))

(fn `UserConstructionScript`)