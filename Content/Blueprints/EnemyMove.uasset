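; EnemyMove is a character Blueprint, apparently an unfinished enemy movement experiment.
; Its only live logic calls AddLocalNavigationGridForBox every Tick with a small box at the actor's location; BeginPlay and the construction script are empty.
; Disconnected nodes hold abandoned attempts using forces, SimpleMoveToActor, interpolated Cube movement and capsule repositioning, none of which run.
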(event `self.ReceiveTick`
  (params (DeltaSeconds :type "Float (single-precision)"))
  (`NavLocalGridManager.AddLocalNavigationGridForBox` (`self.K2_GetActorLocation`) (3.5 4.0 2.0)))

(event `self.ReceiveBeginPlay`)

(fn `UserConstructionScript`)