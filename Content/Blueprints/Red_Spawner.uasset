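; Red Spawner actor for the Death Race game mode that spawns AI_Red pawns at its root location.
; BeginPlay spawns one immediately; Tick then maps the game mode's DifficultySelect (Infinite, Easy, Default, Hard) to a random interval range, with longer intervals on harder settings.
; A shared Delay, which ignores re-triggers while pending, turns Tick into a repeating spawn loop.
; Disconnected per-difficulty spawn chains remain unused.
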(event `self.ReceiveBeginPlay`
  (`AIBlueprintHelperLibrary.SpawnAIFromClass` "/Game/Blueprints/AI_Red.AI_Red_C" null (`SceneComponent.K2_GetComponentLocation` (`self.DefaultSceneRoot`)) (struct) false null))

(event `self.ReceiveTick`
  (params (DeltaSeconds :type "Float (single-precision)"))
  (bind _asdeath_race_game_mode (cast `/Game/GameMode/DeathRaceGameMode` (`GameplayStatics.GetGameMode`)))
  (bind _difficultyselect (`/Game/GameMode/DeathRaceGameMode.DifficultySelect` _asdeath_race_game_mode))
  ;[1 0.9549 0.4007] Check Difficulty Select
  (if (== _difficultyselect 0)
    ;[1 0.5371 0.9012] Infinite
    (set `self.SpawnRateMinimum` 0.0)
    (set `self.SpawnRateMaximum` 2.0)
    ;[0.2544 0.9502 1] Spawner
    (`KismetSystemLibrary.Delay` (`KismetMathLibrary.RandomFloatInRange` (`self.SpawnRateMinimum`) (`self.SpawnRateMaximum`)) :!label _label)
    (`AIBlueprintHelperLibrary.SpawnAIFromClass` "/Game/Blueprints/AI_Red.AI_Red_C" null (`SceneComponent.K2_GetComponentLocation` (`self.DefaultSceneRoot`)) (struct) false null)
    (elif (== _difficultyselect 1)
      ;[0.6151 1 0.4263] Easy
      (set `self.SpawnRateMinimum` 1.0)
      (set `self.SpawnRateMaximum` 2.0)
      (goto _label)
      (elif (== _difficultyselect 2)
        ;[0.4782 0.4475 1] Default
        (set `self.SpawnRateMinimum` 1.0)
        (set `self.SpawnRateMaximum` 4.0)
        (goto _label)
        (elif (== _difficultyselect 3)
          ;[1 0.2312 0.2411] Hard
          (set `self.SpawnRateMinimum` 3.0)
          (set `self.SpawnRateMaximum` 8.0)
          (goto _label))))))

(fn `UserConstructionScript`)