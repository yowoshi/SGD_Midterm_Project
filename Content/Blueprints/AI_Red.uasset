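; AI_Red is a wandering target pawn for a death race game mode that the player destroys for points.
; Tick runs through a random Delay of up to three seconds, then spawns an explosion and issues AIMoveTo to a random reachable point, setting a Moving flag that is never read here.
; Player overlap with the capsule spawns an explosion, destroys the actor and passes AddScore to DeathRaceGameMode's AddTargetPoints.
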(event `self.ReceiveBeginPlay`)

(event `self.ReceiveTick`
  (params (DeltaSeconds :type "Float (single-precision)"))
  (bind _returnvalue (`self.K2_GetActorLocation`))
  ;[1 0.5585 0.8445] AI Movement
  (`KismetSystemLibrary.Delay` (`KismetMathLibrary.RandomFloatInRange` 0.0 3.0))
  (`GameplayStatics.SpawnEmitterAtLocation` "/Game/StarterContent/Particles/P_Explosion.P_Explosion" _returnvalue)
  (set `self.moving` true)
  (`|AIMoveTo` self (`NavigationSystemV1.K2_GetRandomReachablePointInRadius` _returnvalue 5000.0 null null) null
    (:`OnSuccess`
      _)
    (:`OnFail`
      _))
  (set `self.moving` false))

(event `self.CapsuleComponent.OnComponentBeginOverlap`
  (params (OverlappedComponent :type "PrimitiveComponent Object Reference") (OtherActor :type "Actor Object Reference") (OtherComp :type "PrimitiveComponent Object Reference") (OtherBodyIndex :type Integer) (bFromSweep :type Boolean) (SweepResult :type "HitResult Structure (by ref)"))
  ;[0.6734 0.5767 1] Destroys Actor on Overlap and Increases Score by 1
  (if (== OtherActor (`GameplayStatics.GetPlayerPawn` 0))
    (`GameplayStatics.SpawnEmitterAtLocation` "/Game/StarterContent/Particles/P_Explosion.P_Explosion" (`self.K2_GetActorLocation`))
    (`self.K2_DestroyActor`)
    (bind _asdeath_race_game_mode (cast `/Game/GameMode/DeathRaceGameMode` (`GameplayStatics.GetGameMode`)))
    (`/Game/GameMode/DeathRaceGameMode.AddTargetPoints` _asdeath_race_game_mode (`self.Add Score`))))

(fn `UserConstructionScript`)