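; Blue_Spawner is a spawner Blueprint that repeatedly spawns AI_Blue pawns at its scene root location.
; Tick drives latent Delays as a repeating timer, with Easy, Default and Hard branches setting spawn pace.
; Each branch spawns faster until a printed Count reaches its threshold, then continues indefinitely at a slower interval.
; Branch conditions are hardcoded booleans, so only the Default branch runs.
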(event `self.ReceiveTick`
  (params (DeltaSeconds :type "Float (single-precision)"))
  (if false
    _
    (elif false
      ;[0.3284 1 0.3075] Easy
      (if (< (`self.count`) 3)
        (`KismetSystemLibrary.Delay` 10.0)
        (`AIBlueprintHelperLibrary.SpawnAIFromClass` "/Game/Blueprints/AI_Blue.AI_Blue_C" null (`SceneComponent.K2_GetComponentLocation` (`self.DefaultSceneRoot`)) (struct) true null)
        (set `self.count` (+ (`self.count`) 1))
        (`KismetSystemLibrary.PrintString` (`KismetStringLibrary.Conv_IntToString` (`self.count`)))
        (else
          (`KismetSystemLibrary.Delay` 20.0)
          (`AIBlueprintHelperLibrary.SpawnAIFromClass` "/Game/Blueprints/AI_Blue.AI_Blue_C" null (`SceneComponent.K2_GetComponentLocation` (`self.DefaultSceneRoot`)) (struct) true null)))
      (elif true
        ;[0 0.1289 1] Default
        (if (< (`self.count`) 5)
          (`KismetSystemLibrary.Delay` 8.0)
          (`AIBlueprintHelperLibrary.SpawnAIFromClass` "/Game/Blueprints/AI_Blue.AI_Blue_C" null (`SceneComponent.K2_GetComponentLocation` (`self.DefaultSceneRoot`)) (struct) true null)
          (set `self.count` (+ (`self.count`) 1))
          (`KismetSystemLibrary.PrintString` (`KismetStringLibrary.Conv_IntToString` (`self.count`)))
          (else
            (`KismetSystemLibrary.Delay` 20.0)
            (`AIBlueprintHelperLibrary.SpawnAIFromClass` "/Game/Blueprints/AI_Blue.AI_Blue_C" null (`SceneComponent.K2_GetComponentLocation` (`self.DefaultSceneRoot`)) (struct) true null)))
        (elif false
          ;[1 0.1632 0.1174] Hard
          (if (< (`self.count`) 8)
            (`KismetSystemLibrary.Delay` 6.0)
            (`AIBlueprintHelperLibrary.SpawnAIFromClass` "/Game/Blueprints/AI_Blue.AI_Blue_C" null (`SceneComponent.K2_GetComponentLocation` (`self.DefaultSceneRoot`)) (struct) true null)
            (set `self.count` (+ (`self.count`) 1))
            (`KismetSystemLibrary.PrintString` (`KismetStringLibrary.Conv_IntToString` (`self.count`)))
            (else
              (`KismetSystemLibrary.Delay` 15.0)
              (`AIBlueprintHelperLibrary.SpawnAIFromClass` "/Game/Blueprints/AI_Blue.AI_Blue_C" null (`SceneComponent.K2_GetComponentLocation` (`self.DefaultSceneRoot`)) (struct) true null))))))))

(fn `UserConstructionScript`)